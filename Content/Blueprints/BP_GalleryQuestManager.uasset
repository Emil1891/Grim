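; BP_GalleryQuestManager handles narrator audio and mix changes for the gallery's Romeo quest.
; Quest start and completion events play narration through AudioNarrator and push NarratorMix, which is popped when the audio finishes; completion also plays a second 2D success clip.
; Reminder and wrong-person events only push the mix, then pop it repeatedly after fixed delays.
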(event `self.TalkedToWrongPersonEvent`
  (`GameplayStatics.PushSoundMixModifier` "/Game/Audio/Class/NarratorMix.NarratorMix")
  (`KismetSystemLibrary.Delay` 3.0)
  (`GameplayStatics.PopSoundMixModifier` "/Game/Audio/Class/NarratorMix.NarratorMix")
  (`GameplayStatics.PopSoundMixModifier` "/Game/Audio/Class/NarratorMix.NarratorMix")
  (`GameplayStatics.PopSoundMixModifier` "/Game/Audio/Class/NarratorMix.NarratorMix")
  (`GameplayStatics.PopSoundMixModifier` "/Game/Audio/Class/NarratorMix.NarratorMix"))

(event `self.OnReminderStarted`
  (`GameplayStatics.PushSoundMixModifier` "/Game/Audio/Class/NarratorMix.NarratorMix")
  (`KismetSystemLibrary.Delay` 6.0)
  (`GameplayStatics.PopSoundMixModifier` "/Game/Audio/Class/NarratorMix.NarratorMix")
  (`GameplayStatics.PopSoundMixModifier` "/Game/Audio/Class/NarratorMix.NarratorMix")
  (`GameplayStatics.PopSoundMixModifier` "/Game/Audio/Class/NarratorMix.NarratorMix")
  (`GameplayStatics.PopSoundMixModifier` "/Game/Audio/Class/NarratorMix.NarratorMix")
  (`GameplayStatics.PopSoundMixModifier` "/Game/Audio/Class/NarratorMix.NarratorMix")
  (`GameplayStatics.PopSoundMixModifier` "/Game/Audio/Class/NarratorMix.NarratorMix")
  (`GameplayStatics.PopSoundMixModifier` "/Game/Audio/Class/NarratorMix.NarratorMix")
  (`GameplayStatics.PopSoundMixModifier` "/Game/Audio/Class/NarratorMix.NarratorMix"))

(event `self.OnQuestComplete`
  (bind _audionarrator (`self.AudioNarrator`))
  (`AudioComponent.SetSound` _audionarrator "/Game/Audio/SFX/Gallery/Voice/Romeo_Success__Romeo___Juliet_.Romeo_Success__Romeo___Juliet_")
  (`GameplayStatics.PlaySound2D` "/Game/Audio/SFX/Gallery/Voice/Romeo_Success__Callum_.Romeo_Success__Callum_" 1.0 1.0 0.0 null null)
  (`AudioComponent.Play` _audionarrator 0.0)
  (`|ExecutionSequence` :!label _label
    (:`then_0`
      (`GameplayStatics.PushSoundMixModifier` "/Game/Audio/Class/NarratorMix.NarratorMix"))
    (:`then_1`
      (add `AudioComponent.OnAudioFinished` _audionarrator (delegate `NarrationFinished`))
      (add `AudioComponent.OnAudioFinished` (`self.AudioNarrator`) (delegate `NarrationFinished`)))))

(event `self.OnQuestStarted`
  (bind _audionarrator (`self.AudioNarrator`))
  (`AudioComponent.SetSound` _audionarrator "/Game/Audio/SFX/Gallery/Voice/Romeo_Giving_Quest__Callum_.Romeo_Giving_Quest__Callum_")
  (`AudioComponent.Play` _audionarrator 0.0)
  (goto _label))

(event `NarrationFinished`
  (`GameplayStatics.PopSoundMixModifier` "/Game/Audio/Class/NarratorMix.NarratorMix"))

(fn `UserConstructionScript`)
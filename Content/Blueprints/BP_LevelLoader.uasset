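; Level transition actor that opens LevelToLoad when a GrimCharacter overlaps it.
; With a valid SoundToPlay, it plays the 2D sound, waits out its duration, then sets ExitTriggered and opens the level after FadeTime.
; While ExitTriggered, Tick lowers the Master sound class volume through a MasterFadeMix override to fade audio out.
; Without a sound, the level opens immediately with no fade.
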(event `self.ReceiveTick`
  (params (DeltaSeconds :type "Float (single-precision)"))
  (bind _returnvalue (- (`self.VolumeToSet`) (/ DeltaSeconds (`self.FadeTime`))))
  (if (`self.ExitTriggered`)
    (bind _output_get (set `self.VolumeToSet` _returnvalue))
    (if (> _returnvalue 0.0)
      (`GameplayStatics.SetSoundMixClassOverride` "/Game/Audio/Class/MasterFadeMix.MasterFadeMix" "/Engine/EngineSounds/Master.Master" _output_get 1.0 0.0)
      (`GameplayStatics.PushSoundMixModifier` "/Game/Audio/Class/MasterFadeMix.MasterFadeMix"))))

(event `self.ReceiveActorBeginOverlap`
  (params (OtherActor :type "Actor Object Reference"))
  (bind _soundtoplay (`self.SoundToPlay`))
  (cast `GrimCharacter` OtherActor)
  (if (`KismetSystemLibrary.IsValid` (`self.SoundToPlay`))
    (`GameplayStatics.PlaySound2D` _soundtoplay 1.0 1.0 0.0 null null)
    (`KismetSystemLibrary.Delay` (`SoundBase.Duration` _soundtoplay))
    (set `self.ExitTriggered` true)
    (`KismetSystemLibrary.Delay` (`self.FadeTime`))
    (`GameplayStatics.OpenLevel` (`self.LevelToLoad`))
    (else
      (`GameplayStatics.OpenLevel` (`self.LevelToLoad`)))))

(fn `UserConstructionScript`)
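; BP_CryptGramophone is a gramophone that plays attached music from BeginPlay and reacts when a GrimCharacter overlaps it.
; Before the last entry in its Positions list, an overlap plays a concurrency-controlled 2D reset cue and calls MoveCurrentPosition to relocate it.
; At the last position, it only prints a Swedish placeholder for ending narration and a level change.
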(event `self.ReceiveActorBeginOverlap`
  (params (OtherActor :type "Actor Object Reference"))
  (bind _asgrim_character (cast `GrimCharacter` OtherActor))
  (if (== (`self.CurrentPosition`) (`KismetArrayLibrary.Array_LastIndex` (`self.Positions`)))
    (`KismetSystemLibrary.PrintString` "SPELA ENDING NARRATION OCH BYT NIVÅ")
    (else
      (`GameplayStatics.PlaySound2D` "/Game/Audio/JoakimAudio/GramophoneResetCue.GramophoneResetCue" 1.0 1.0 0.0 "/Game/Audio/JoakimAudio/GramophoneConcurrency.GramophoneConcurrency" _asgrim_character)
      (`self.MoveCurrentPosition`))))

(event `self.ReceiveBeginPlay`
  (`GameplayStatics.SpawnSoundAttached` "/Game/Audio/JoakimAudio/GramophoneMusicCue.GramophoneMusicCue" (`self.Cube`) "None" (0.0 0.0 0.0) (struct) "KeepRelativeOffset" false 1.0 1.0 0.0 "/Game/Audio/Attenuation/GuidingAttenuation.GuidingAttenuation" "/Game/Audio/JoakimAudio/GramophoneConcurrency.GramophoneConcurrency"))

(fn `UserConstructionScript`)
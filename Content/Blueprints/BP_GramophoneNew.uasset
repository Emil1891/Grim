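; Gramophone actor that starts its attached audio components, all except GramophoneMusic, with a shared facade attenuation setting.
; On BeginPlay it loops over every other AudioComponent, assigns AttenuationGramophoneFacade, plays it from the start and disables actor tick.
; Tick repeats the identical pass, so it serves as a fallback that runs until such a component is found and ticking switches off.
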(event `self.ReceiveBeginPlay`
  (for _array_element (`self.K2_GetComponentsByClass` "/Script/Engine.AudioComponent")
    (if (!= _array_element (`self.GramophoneMusic`))
      (set `AudioComponent.AttenuationSettings` "/Game/Audio/Attenuation/AttenuationGramophoneFacade.AttenuationGramophoneFacade" _array_element)
      (`AudioComponent.Play` _array_element 0.0)
      (`self.SetActorTickEnabled` false))))

(event `self.ReceiveTick`
  (params (DeltaSeconds :type "Float (single-precision)"))
  (for _array_element (`self.K2_GetComponentsByClass` "/Script/Engine.AudioComponent")
    (if (!= _array_element (`self.GramophoneMusic`))
      (set `AudioComponent.AttenuationSettings` "/Game/Audio/Attenuation/AttenuationGramophoneFacade.AttenuationGramophoneFacade" _array_element)
      (`AudioComponent.Play` _array_element 0.0)
      (`self.SetActorTickEnabled` false))))

(fn `UserConstructionScript`)